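; Moving platform that travels through an ordered array of waypoint actors, with externally callable Start and Stop functions.
; BeginPlay hides the waypoints, and the construction script applies the chosen mesh and material.
; A rate-scaled timeline lerps between waypoint positions, and its event track advances to the next segment.
; At the last waypoint it either ends or, with Loop set, restarts from the first, snapping back rather than reversing.
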(event Custom|Platform%20Start
  (bind _motion_timeline (Variables|Default|Getmotion%20timeline))
  (CallFunction|SetFirstWaypoint)
  (Components|Timeline|SetPlayRate _motion_timeline (Variables|Default|Getrate))
  (Components|Timeline|PlayfromStart _motion_timeline))

(event EventBeginPlay
  ;[1 1 1] makes platform points invisible
  (for _array_element (Variables|Default|Getwaypoints)
    (Rendering|SetActorHiddenInGame _array_element true)))

(fn ConstructionScript
  (bind _platform_mesh (Variables|Default|Getplatform%20mesh))
  (Components|StaticMesh|SetStaticMesh _platform_mesh (Variables|Default|Getstatic_mesh))
  (Rendering|Material|SetMaterial _platform_mesh 0 (Variables|Default|Getmaterial)))

(fn SetPositions
  (bind _waypoints (Variables|Default|Getwaypoints))
  (Variables|Default|Setcurrent%20waypoint%20pos (Transformation|GetActorLocation (Utilities|Array|Get(acopy) _waypoints (Variables|Default|Getcurrent%20waypoint%20index))))
  (Variables|Default|Setnext%20waypoint%20pos (Transformation|GetActorLocation (Utilities|Array|Get(acopy) _waypoints (Variables|Default|Getnext%20waypoint%20index)))))

(fn SetFirstWaypoint
  (Variables|Default|Setcurrent%20waypoint%20index 0)
  (Variables|Default|Setnext%20waypoint%20index 1)
  (CallFunction|SetPositions))

(fn SetNextWaypoint
  (bind _result (Math|Integer|IncrementInt (Variables|Default|Getcurrent%20waypoint%20index))
    (:%20%20
      (Variables|Default|Setnext%20waypoint%20index (+ _result 1))
      (CallFunction|SetPositions))))

(fn PathIsFin
  (return (== (Variables|Default|Getnext%20waypoint%20index) (- (Utilities|Array|Length (Variables|Default|Getwaypoints)) 1))))

(fn Start
  (CallFunction|PlatformStart))

(fn Stop
  (Audio|Components|Audio|Stop (Variables|Default|Getmotion%20timeline)))