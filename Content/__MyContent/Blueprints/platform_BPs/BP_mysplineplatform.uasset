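; Spline-following moving platform whose mesh travels along a spline, starting on BeginPlay.
; A timeline, with play rate set from a Rate variable, outputs a normalized distance that is scaled by spline length to place the mesh in world space without sweep.
; The construction script applies the configurable static mesh and material to the platform.
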(event Custom|platform%20start
  (Components|Timeline|SetPlayRate (Variables|Default|Getmotion%20timeline) (Variables|Default|Getrate))
  (bind _spline_distance (Timeline|motion%20timeline PlayFromStart)
    (:Update
      (Transformation|SetWorldLocation (Variables|Default|Getplatform%20mesh) (Spline|GetLocationatDistanceAlongSpline (Variables|Default|GetSpline) (* _spline_distance (Spline|GetSplineLength (Variables|Default|GetSpline))) "World") false false))))

(event EventBeginPlay
  (CallFunction|PlatformStart))

(fn ConstructionScript
  (bind _platform_mesh (Variables|Default|Getplatform%20mesh))
  (Components|StaticMesh|SetStaticMesh _platform_mesh (Variables|Default|Getstatic%20mesh))
  (Rendering|Material|SetMaterial _platform_mesh 0 (Variables|Default|Getmaterial)))